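; Spore zone Blueprint that changes the FirstPersonCharacter player's health: despite the Damage_Spores name, health rises inside the zone and drains outside it.
; DamageBox begin and end overlaps toggle IsInSpores without checking which actor overlaps.
; Tick reads the flag and uses short Delays to throttle the health changes, with the drain outside larger than the gain inside.
; Health is written directly on player 0's character, with no clamping here.
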(event `self.ReceiveBeginPlay`
  (set `self.IsInSpores` false))

(event `self.Damage Box.OnComponentBeginOverlap`
  (params (OverlappedComponent :type "PrimitiveComponent Object Reference") (OtherActor :type "Actor Object Reference") (OtherComp :type "PrimitiveComponent Object Reference") (OtherBodyIndex :type Integer) (bFromSweep :type Boolean) (SweepResult :type "HitResult Structure (by ref)"))
  (set `self.IsInSpores` true))

(event `self.Damage Box.OnComponentEndOverlap`
  (params (OverlappedComponent :type "PrimitiveComponent Object Reference") (OtherActor :type "Actor Object Reference") (OtherComp :type "PrimitiveComponent Object Reference") (OtherBodyIndex :type Integer))
  (set `self.IsInSpores` false))

(event `self.ReceiveTick`
  (params (DeltaSeconds :type "Float (single-precision)"))
  (if (`self.IsInSpores`)
    (`KismetSystemLibrary.Delay` 0.2)
    (bind _asfirst_person_character (cast `/Game/FirstPersonBP/Blueprints/FirstPersonCharacter` (`GameplayStatics.GetPlayerCharacter` 0)))
    (set `/Game/FirstPersonBP/Blueprints/FirstPersonCharacter.Health` (+ (`/Game/FirstPersonBP/Blueprints/FirstPersonCharacter.Health` _asfirst_person_character) 5) _asfirst_person_character)
    (else
      (`KismetSystemLibrary.Delay` 0.2)
      (bind _asfirst_person_character_2 (cast `/Game/FirstPersonBP/Blueprints/FirstPersonCharacter` (`GameplayStatics.GetPlayerCharacter` 0)))
      (set `/Game/FirstPersonBP/Blueprints/FirstPersonCharacter.Health` (- (`/Game/FirstPersonBP/Blueprints/FirstPersonCharacter.Health` _asfirst_person_character_2) 10) _asfirst_person_character_2))))

(fn `UserConstructionScript`)