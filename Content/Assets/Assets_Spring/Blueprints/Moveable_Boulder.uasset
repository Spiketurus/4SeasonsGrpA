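; Moveable_Boulder is a boulder actor that gets shoved along the X or Y axis when something overlaps one of its four side trigger boxes.
; Each box stores a fixed offset pointing away from its side, and a shared step adds it to the actor's location.
; The move is a single instant jump in world axes without sweep, and the overlapping actor is not filtered.
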(event `self.YNegBox.OnComponentBeginOverlap`
  (params (OverlappedComponent :type "PrimitiveComponent Object Reference") (OtherActor :type "Actor Object Reference") (OtherComp :type "PrimitiveComponent Object Reference") (OtherBodyIndex :type Integer) (bFromSweep :type Boolean) (SweepResult :type "HitResult Structure (by ref)"))
  (set `self.Boulder Position Movement` (0.0 50.0 0.0))
  (`self.K2_SetActorLocation` (+ (`self.K2_GetActorLocation`) (`self.Boulder Position Movement`)) :!label _label))

(event `self.YPosBox.OnComponentBeginOverlap`
  (params (OverlappedComponent :type "PrimitiveComponent Object Reference") (OtherActor :type "Actor Object Reference") (OtherComp :type "PrimitiveComponent Object Reference") (OtherBodyIndex :type Integer) (bFromSweep :type Boolean) (SweepResult :type "HitResult Structure (by ref)"))
  (set `self.Boulder Position Movement` (0.0 -50.0 0.0))
  (goto _label))

(event `self.XNegBox.OnComponentBeginOverlap`
  (params (OverlappedComponent :type "PrimitiveComponent Object Reference") (OtherActor :type "Actor Object Reference") (OtherComp :type "PrimitiveComponent Object Reference") (OtherBodyIndex :type Integer) (bFromSweep :type Boolean) (SweepResult :type "HitResult Structure (by ref)"))
  (set `self.Boulder Position Movement` (50.0 0.0 0.0))
  (goto _label))

(event `self.XPosBox.OnComponentBeginOverlap`
  (params (OverlappedComponent :type "PrimitiveComponent Object Reference") (OtherActor :type "Actor Object Reference") (OtherComp :type "PrimitiveComponent Object Reference") (OtherBodyIndex :type Integer) (bFromSweep :type Boolean) (SweepResult :type "HitResult Structure (by ref)"))
  (set `self.Boulder Position Movement` (-50.0 0.0 0.0))
  (goto _label))

(fn `UserConstructionScript`)